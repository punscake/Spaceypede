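; Player controller for the main menu that shows the menu widget and the mouse cursor on BeginPlay.
; It exposes events for hosting and for finding and joining a game, with hosting relayed from a client event to a server call.
; Both the host and join events cast the game instance to SteamGameInstance and delegate the work to it, passing the controller itself.
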(event `self.ReceiveBeginPlay`
  (bind _returnvalue (`|CreateWidget` "/Game/Widgets/MainMenuWG.MainMenuWG_C" self))
  (`UserWidget.AddToViewport` _returnvalue 0)
  (set `self.bShowMouseCursor` true))

(event `Client_HostGame`
  (`self.Server_HostGame`))

(event `Server_HostGame`
  (bind _assteam_game_instance (cast `/Game/SteamGameInstance` (`GameplayStatics.GetGameInstance`)))
  (`/Game/SteamGameInstance.Host` _assteam_game_instance self))

(event `FindAndJoinFirst`
  (bind _assteam_game_instance (cast `/Game/SteamGameInstance` (`GameplayStatics.GetGameInstance`)))
  (`/Game/SteamGameInstance.Join` _assteam_game_instance self))

(fn `UserConstructionScript`)